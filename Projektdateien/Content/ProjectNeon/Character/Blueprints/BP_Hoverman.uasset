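; BP_Hoverman is the player's hover character Blueprint, adding camera, feedback and crouch handling to inherited movement events.
; BeginPlay spawns BP_CameraManager above it as the view target and binds dash, trick and wall-bounce delegates.
; These delegates play sounds, with dash and trick also flashing DashFX on short timers.
; Crouch events resize the capsule and crouch start offsets the mesh, while timer events forward to StartTimer and StopTimer.
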(event Custom|Starting%20Timer
  (Class|ProjectNeonCharacter|StartTimer))

(event Custom|OnDashPerformed_Event
  ;[1 1 1] Dash Binding
  (Components|Activation|SetActive (Variables|Default|GetDashFX) true true)
  (Utilities|Time|SetTimerbyEvent (delegate Custom|OnDashEnd) 0.25)
  (Audio|PlaySound2D "/Game/ProjectNeon/Maps/Audio/Sound/A_BoostSound_Cue.A_BoostSound_Cue" 1.0 1.0 0.0 0 0))

(event Custom|CustomEvent
  ;[1 1 1] Trick Binding
  (Components|Activation|SetActive (Variables|Default|GetDashFX) false false))

(event Custom|End%20Timer
  (params (LevelIdx :type Integer))
  (Class|ProjectNeonCharacter|StopTimer LevelIdx))

(event Custom|OnTrickPerformed_Event
  ;[1 1 1] Trick Binding
  (Components|Activation|SetActive (Variables|Default|GetDashFX) true true)
  (Utilities|Time|SetTimerbyEvent (delegate Custom|CustomEvent) 0.15)
  (Audio|PlaySound2D "/Game/ProjectNeon/Maps/Audio/Sound/A_TrickSound_2_Cue.A_TrickSound_2_Cue" 1.0 1.0 0.0 0 0))

(event Custom|OnDashEnd
  ;[1 1 1] Dash Binding
  (Components|Activation|SetActive (Variables|Default|GetDashFX) false false))

(event Custom|OnBounceCollison_Event
  ;[1 1 1] BounceCollision Binding
  (Audio|PlaySound2D "/Game/ProjectNeon/Maps/Audio/Sound/A_BounceSound_Cue.A_BounceSound_Cue" 1.0 1.0 0.0 0 0))

(event EventBeginPlay
  (bind _returnvalue (Transformation|GetActorLocation))
  ;[1 1 1] Initialize Camera Manager
  (bind _returnvalue_2 (Game|SpawnActorfromClass "/Game/ProjectNeon/Character/Blueprints/BP_CameraManager.BP_CameraManager_C" (Math|Transform|MakeTransform (Math|Vector|MakeVector (.x _returnvalue) (.y _returnvalue) (+ (.z _returnvalue) (Variables|Default|GetCameraHeightOffset))) "0, 0, 0" "1.000000,1.000000,1.000000") "Undefined" "MultiplyWithRoot" 0 self 0))
  (Game|Player|SetViewTargetwithBlend (Game|GetPlayerController 0) _returnvalue_2 0.0 "VTBlend_Linear" 0.0 false)
  (Physics|SetSimulatePhysics (Variables|Default|GetCapsuleComponent) false)
  ;[1 1 1] Dash Binding
  (EventDispatchers|AssignOnDashPerformed (delegate Custom|OnDashPerformed_Event))
  ;[1 1 1] Trick Binding
  (EventDispatchers|AssignOnTrickPerformed (delegate Custom|OnTrickPerformed_Event))
  ;[1 1 1] BounceCollision Binding
  (EventDispatchers|BindEventtoOnBouncyWallCollision (delegate Custom|OnBounceCollison_Event)))

(event EventOnStartCrouch
  (params (HalfHeightAdjust :type Float%20%28single-precision%29) (ScaledHalfHeightAdjust :type Float%20%28single-precision%29))
  (bind _capsulecomponent (Variables|Default|GetCapsuleComponent))
  ;[1 1 1] Change Skelet while Crouching
  (Transformation|SetRelativeLocation (Variables|Character|GetMesh) (Math|Vector|MakeVector 0.0 0.0 (* (.OutHalfHeight (Components|Capsule|GetScaledCapsuleSize (Variables|Default|GetCapsuleComponent))) -2.26)) false false)
  (Components|Capsule|SetCapsuleRadius _capsulecomponent 5.0 true)
  (Components|Capsule|SetCapsuleHalfHeight _capsulecomponent 5.0 true))

(event EventOnEndCrouch
  (params (HalfHeightAdjust :type Float%20%28single-precision%29) (ScaledHalfHeightAdjust :type Float%20%28single-precision%29))
  (bind _capsulecomponent (Variables|Default|GetCapsuleComponent))
  ;[1 1 1] Change Skelet after Crouching
  (Components|Capsule|SetCapsuleRadius _capsulecomponent 35.0 true)
  (Components|Capsule|SetCapsuleHalfHeight _capsulecomponent 9e+01 true))

(fn ConstructionScript)