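; BP_Finishline is the finish-line trigger that ends the player's timed run in a level.
; On BeginPlay it caches the player's BP_Hoverman pawn and maps the current level name (Level 1 to 3) to a level index.
; When its collision component begins an overlap, it calls EndTimer on the cached Hoverman with that index and plays a 2D finish sound, without checking which actor overlapped.
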(event OnComponentBeginOverlap(Finishlinie)
  (params (OverlappedComponent :type Primitive%20Component%20Object%20Reference) (OtherActor :type Actor%20Object%20Reference) (OtherComp :type Primitive%20Component%20Object%20Reference) (OtherBodyIndex :type Integer) (bFromSweep :type Boolean) (SweepResult :type Hit%20Result%20Structure%20%28by%20ref%29))
  (Default|EndTimer (Variables|Default|GetAs%20BP%20Hoverman) (Variables|Default|GetLvlIdx))
  (Audio|PlaySound2D "/Game/ProjectNeon/Maps/Audio/Sound/A_FinishSound_Cue.A_FinishSound_Cue" 1.0 1.0 0.0 0 0))

(event EventBeginPlay
  (bind _asbp_hoverman (Utilities|Casting|CastToBP_Hoverman (Game|Player|GetPlayerPawn 0)))
  (Variables|Default|SetAs%20BP%20Hoverman _asbp_hoverman)
  (bind _returnvalue (Game|GetCurrentLevelName true))
  (switch string _returnvalue
    (:Level_1
      (Variables|Default|SetLvlIdx 0))
    (:Level_2
      (Variables|Default|SetLvlIdx 1))
    (:Level_3
      (Variables|Default|SetLvlIdx 2))))

(fn ConstructionScript)