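; BP_Neon is a neon prop that flickers irregularly by swapping its static mesh material between M_Neon and M_BlackMetal.
; Each Tick adds delta time to a running timer and triggers a FlipFlop when that timer modulo a random float is near zero.
; IsOn toggles with each swap to choose the random range, so the neon material tends to hold longer than the brief dark blinks.
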(event EventBeginPlay
  (Variables|Default|SetNewVar 0.0)
  (Variables|Default|SetisOn true))

(event Collision|EventActorBeginOverlap
  (params (OtherActor :type Actor%20Object%20Reference)))

(event EventTick
  (params (DeltaSeconds :type Float%20%28single-precision%29))
  (bind _staticmesh (Variables|Default|GetStaticMesh))
  (if (Variables|Default|GetisOn)
    (Variables|Default|SetMax 0.3)
    (Variables|Default|SetMin 0.0)
    (else
      (Variables|Default|SetMax 3.0)
      (Variables|Default|SetMin 1.0)))
  (bind _output_get (Variables|Default|SetNewVar (+ (Utilities|Time|GetWorldDeltaSeconds) (Variables|Default|GetNewVar))))
  (if (< (Math|Float|%(Float) _output_get (Math|Random|RandomFloatinRange (Variables|Default|GetMin) (Variables|Default|GetMax))) 0.01)
    (Utilities|FlowControl|FlipFlop
      (:A
        (Rendering|Material|SetMaterial _staticmesh 0 "/Game/ProjectNeon/Materials/M_Neon.M_Neon"))
      (:B
        (Rendering|Material|SetMaterial _staticmesh 0 "/Game/ProjectNeon/Materials/M_BlackMetal.M_BlackMetal")))
    (Variables|Default|SetisOn (not (Variables|Default|GetisOn)))))

(fn ConstructionScript)